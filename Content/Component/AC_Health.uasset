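; Health component that tracks an owning actor's health and death state.
; BeginPlay clamps max health, fills health to it and makes the owner damageable.
; HandleOwnerDamage subtracts positive damage while alive; at zero it marks death, disables the owner's damage and player 0 input, then fires OnDeath, before OnHealthChanged.
; No binding for the handler appears here, and an unreachable copy of its logic remains.
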(event `self.ReceiveBeginPlay`
  (set `self.MaxHealth` (`KismetMathLibrary.FClamp` (`self.MaxHealth`) 1.0 1000000.0))
  (set `self.Health` (`self.MaxHealth`))
  (set `self.bIsDead` false)
  (set `Actor.bCanBeDamaged` true (`self.GetOwner`)))

(fn `HandleOwnerDamage`
  (params (DamagedActor :type "Actor Object Reference") (Damage :type "Float (double-precision)") (DamageType :type "DamageType Object Reference") (InstigatedBy :type "Controller Object Reference") (DamageCauser :type "Actor Object Reference"))
  (if (and (> Damage 0.0) (not (`self.bIsDead`)))
    (set `self.Health` (`KismetMathLibrary.FClamp` (- (`self.Health`) Damage) 0.0 (`self.MaxHealth`)))
    (if (<= (`self.Health`) 0.0)
      (set `self.bIsDead` true)
      (set `Actor.bCanBeDamaged` false (`self.GetOwner`))
      (`Actor.DisableInput` (`self.GetOwner`) (`GameplayStatics.GetPlayerController` 0))
      (`self.OnDeath`))
    (`self.OnHealthChanged`)))