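; Sword-wielding Mover-based enemy that attacks a given target, shows its health as text and ragdolls on death.
; TryEnemyAttack checks state, range and cooldown, snaps yaw to the target, then alternates two combo montages.
; While attacking and AC_Combat's trace flag is on, Tick box-traces the blade, damaging only that target, once per swing, if unobstructed.
; HealthComponent processes incoming damage, which cancels attacks, stops movement and triggers a hit reaction or ragdoll.
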(event `self.ReceiveBeginPlay`
  (`parent.ReceiveBeginPlay`)
  (`self.InitializeEnemy`))

(event `self.NPC_GetupCheck`)

(event `self.ReceiveTick`
  (params (DeltaSeconds :type "Float (single-precision)"))
  (`parent.ReceiveTick` DeltaSeconds)
  (`self.UpdateEnemyCombat`))

(event `self.ReceiveAnyDamage`
  (params (Damage :type "Float (single-precision)") (DamageType :type "DamageType Object Reference") (InstigatedBy :type "Controller Object Reference") (DamageCauser :type "Actor Object Reference"))
  (`self.ReceiveCombatDamage` Damage DamageType InstigatedBy DamageCauser))

(event `PlayHitReaction`
  (`|PlayMontageOnMoverActor` (`self.CharacterMover`) "/Game/UEFNAnimations/GaspSword/Anim_DK_Hit_Back_RM_Montage.Anim_DK_Hit_Back_RM_Montage"))

(event `PlayEnemyAttackAnim`
  (`|PlayMontageOnMoverActor` (`self.CharacterMover`) (`self.AttackMontage`)
    (:`OnCompleted`
      (`self.FinishEnemyAttack`))
    (:`OnInterrupted`
      (`self.FinishEnemyAttack`))))

(fn `CancelEnemyAttack`
  (`self.FinishEnemyAttack`)
  (`AnimInstance.Montage_Stop` (`SkeletalMeshComponent.GetAnimInstance` (`self.SkeletalMesh`)) 0.1 (`self.AttackMontage`)))

(fn `EquipEnemySword`
  (bind _returnvalue (`|SpawnActorFromClass` "/Game/Component/BP_Sword.BP_Sword_C" (`self.GetTransform`) "AlwaysSpawn" "MultiplyWithRoot" self null))
  (set `self.EnemyWeapon` _returnvalue)
  (`self.K2_AttachToComponent` _returnvalue (`self.SkeletalMesh`) "Weapon" "SnapToTarget" "SnapToTarget" "SnapToTarget" true)
  (bind _asstatic_mesh_component (cast `StaticMeshComponent` (`self.GetComponentByClass` _returnvalue "/Script/Engine.StaticMeshComponent")))
  (set `self.EnemyWeaponMesh` _asstatic_mesh_component))

(fn `FinishEnemyAttack`
  (`self.SetEnemyWeaponTrace` false)
  (set `self.IsAttacking` false)
  (set `self.NextAttackTime` (+ (`GameplayStatics.GetTimeSeconds`) (`self.AttackCooldown`))))

(fn `InitializeEnemy`
  (`ActorComponent.SetComponentTickEnabled` (`self.GetComponentByClass` self "/Game/Component/AC_Combat.AC_Combat_C") false)
  (`PrimitiveComponent.SetCollisionResponseToChannel` (`self.Capsule`) "ECC_Visibility" "ECR_Block")
  (`SceneComponent.K2_SetRelativeRotation` :`self` (`self.HealthText`))
  (`TextRenderComponent.K2_SetText` (`self.HealthText`) (`KismetTextLibrary.Conv_StringToText` "Enemigo: 100 / 100"))
  (`self.EquipEnemySword`))

(fn `IsEnemyDead`
  (returns (Result :type Boolean) (ReactingToHit :type Boolean) (Attacking :type Boolean))
  (return (`/Game/Component/AC_Health.bIsDead` (`self.HealthComponent`)) (`AnimInstance.Montage_IsPlaying` (`SkeletalMeshComponent.GetAnimInstance` (`self.SkeletalMesh`)) "/Game/UEFNAnimations/GaspSword/Anim_DK_Hit_Back_RM_Montage.Anim_DK_Hit_Back_RM_Montage") (`self.IsAttacking`)))

(fn `IsReactingToHit`
  (returns (Result :type Boolean))
  (return (`AnimInstance.Montage_IsPlaying` (`SkeletalMeshComponent.GetAnimInstance` (`self.SkeletalMesh`)) "/Game/UEFNAnimations/GaspSword/Anim_DK_Hit_Back_RM_Montage.Anim_DK_Hit_Back_RM_Montage")))

(fn `PerformEnemyWeaponTrace`
  (bind _returnvalue (`KismetMathLibrary.MakeVector` 10.0 10.0 10.0))
  (bind _returnvalue_2 (`SceneComponent.GetSocketLocation` (`self.EnemyWeaponMesh`) "TopTrace"))
  (bind _returnvalue_3 (`SceneComponent.GetSocketLocation` (`self.EnemyWeaponMesh`) "BottomTrace"))
  (if (`/Game/Component/AC_Combat.BWeaponTrace` (`self.GetComponentByClass` self "/Game/Component/AC_Combat.AC_Combat_C"))
    (`/Engine/EditorBlueprintResources/StandardMacros.IsValid` (`self.EnemyWeaponMesh`)
      (:`Is Valid`
        (bind (_outhit _returnvalue_4) (`KismetSystemLibrary.BoxTraceSingleForObjects` _returnvalue_2 _returnvalue_3 _returnvalue (struct) (`|MakeArray` "ObjectTypeQuery3" :!type "EObjectTypeQuery Enum") false (`self.ActorsHitThisAttack`)))
        (if _returnvalue_4
          (bind (_bblockinghit _binitialoverlap _time _distance _location _impactpoint _normal _impactnormal _physmat _hitactor) (`GameplayStatics.BreakHitResult` _outhit))
          (if (== _hitactor (`self.AttackTarget`))
            (bind (_outhit_2 _returnvalue_5) (`KismetSystemLibrary.BoxTraceSingle` _returnvalue_2 _returnvalue_3 _returnvalue (struct) "TraceTypeQuery1" false (`self.ActorsHitThisAttack`)))
            (if (or (not _returnvalue_5) (<= _distance (`.Distance` (`GameplayStatics.BreakHitResult` _outhit_2))))
              (`KismetArrayLibrary.Array_AddUnique` (`self.ActorsHitThisAttack`) _hitactor)
              (`GameplayStatics.ApplyDamage` _hitactor (`self.EnemyWeaponDamage`) (`self.GetController`) (`self.EnemyWeapon`)))))))))

(fn `ReceiveCombatDamage`
  (params (Damage :type "Float (double-precision)") (DamageType :type "DamageType Object Reference") (InstigatedBy :type "Controller Object Reference") (DamageCauser :type "Actor Object Reference"))
  (locals (HealthBeforeHit :type "Float (double-precision)"))
  (bind _healthcomponent (`self.HealthComponent`))
  (set `local.HealthBeforeHit` (`/Game/Component/AC_Health.Health` _healthcomponent))
  (`/Game/Component/AC_Health.HandleOwnerDamage` _healthcomponent self Damage DamageType InstigatedBy DamageCauser)
  (if (< (`/Game/Component/AC_Health.Health` _healthcomponent) (`local.HealthBeforeHit`))
    (`self.CancelEnemyAttack`)
    (`self.StopCombatMovement`)
    (`TextRenderComponent.K2_SetText` (`self.HealthText`) (`KismetTextLibrary.Conv_StringToText` (`KismetStringLibrary.BuildString_Double` "" "Vida: " (`/Game/Component/AC_Health.Health` _healthcomponent) " / 100")))
    (if (`/Game/Component/AC_Health.bIsDead` _healthcomponent)
      (`SceneComponent.SetVisibility` (`self.HealthText`) false false)
      (`self.TriggerRagdoll` self true (`self.DefaultRagdollMontageBlendOut`) "NewEnumerator5")
      (else
        (`self.PlayHitReaction`)))))

(fn `SetEnemyWeaponTrace`
  (params (Enabled :type Boolean))
  (set `self.WeaponTraceActive` Enabled)
  (`/Game/Component/AC_Combat.CallToggleWeaponTrace` (`self.GetComponentByClass` self "/Game/Component/AC_Combat.AC_Combat_C") Enabled))

(fn `StopCombatMovement`
  (bind _returnvalue (`self.GetController`))
  (`/Engine/EditorBlueprintResources/StandardMacros.IsValid` _returnvalue
    (:`Is Valid`
      (`Controller.StopMovement` _returnvalue))))

(fn `TryEnemyAttack`
  (params (Target :type "Actor Object Reference"))
  (bind _returnvalue (`KismetMathLibrary.MakeRotator` 0.0 0.0 (.yaw (`KismetMathLibrary.FindLookAtRotation` (`self.K2_GetActorLocation`) (`self.K2_GetActorLocation` Target)))))
  (bind (_result _reactingtohit) (`self.IsEnemyDead`))
  (if (and (not _result) (and (not _reactingtohit) (and (not (`self.IsAttacking`)) (>= (`GameplayStatics.GetTimeSeconds`) (`self.NextAttackTime`)))))
    (`/Engine/EditorBlueprintResources/StandardMacros.IsValid` Target
      (:`Is Valid`
        (if (<= (`self.GetDistanceTo` self Target) (`self.AttackRange`))
          (`self.StopCombatMovement`)
          (set `self.AttackTarget` Target)
          (`self.K2_SetActorRotation` self _returnvalue false)
          (`MoverComponent.K2_QueueInstantMovementEffect` (`self.CharacterMover`) (make `TeleportEffect` (`self.K2_GetActorLocation`) false _returnvalue))
          (`Controller.SetControlRotation` (`self.GetController`) _returnvalue)
          (`self.SetEnemyWeaponTrace` false)
          (`KismetArrayLibrary.Array_Clear` (`self.ActorsHitThisAttack`))
          (`KismetArrayLibrary.Array_AddUnique` (`self.ActorsHitThisAttack`) self)
          (`KismetArrayLibrary.Array_AddUnique` (`self.ActorsHitThisAttack`) (`self.EnemyWeapon`))
          (set `self.IsAttacking` true)
          (if (== (`self.AttackComboIndex`) 0)
            (set `self.AttackMontage` "/Game/UEFNAnimations/GaspSword/Montages/Anim_PS_Combo_A1_RM_Montage.Anim_PS_Combo_A1_RM_Montage")
            (set `self.AttackComboIndex` 1)
            (else
              (set `self.AttackMontage` "/Game/UEFNAnimations/GaspSword/Montages/Anim_PS_Combo_A2_RM_Montage.Anim_PS_Combo_A2_RM_Montage")
              (set `self.AttackComboIndex` 0)))
          (`self.PlayEnemyAttackAnim`))))))

(fn `UpdateEnemyCombat`
  (if (and (`self.IsAttacking`) (not (`/Game/Component/AC_Health.bIsDead` (`self.HealthComponent`))))
    (`self.PerformEnemyWeaponTrace`)))

(fn `UserConstructionScript`
  (`parent.UserConstructionScript`))