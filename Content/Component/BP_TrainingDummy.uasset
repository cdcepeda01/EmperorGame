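; BP_TrainingDummy is a damageable training dummy actor that shows its health on a text label.
; Its AnyDamage event forwards hits to a HealthComponent, then rewrites HealthText from the component's Health against a hardcoded maximum.
; The dummy destroys itself once the component reports death; display strings are hardcoded in Spanish.
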(event `self.ReceiveBeginPlay`
  (`TextRenderComponent.K2_SetText` (`self.HealthText`) (`KismetTextLibrary.Conv_StringToText` "Entrenamiento: 100 / 100")))

(event `self.ReceiveAnyDamage`
  (params (Damage :type "Float (single-precision)") (DamageType :type "DamageType Object Reference") (InstigatedBy :type "Controller Object Reference") (DamageCauser :type "Actor Object Reference"))
  (bind _healthcomponent (`self.HealthComponent`))
  (`/Game/Component/AC_Health.HandleOwnerDamage` _healthcomponent self Damage DamageType InstigatedBy DamageCauser)
  (`TextRenderComponent.K2_SetText` (`self.HealthText`) (`KismetTextLibrary.Conv_StringToText` (`KismetStringLibrary.BuildString_Double` "" "Vida: " (`/Game/Component/AC_Health.Health` _healthcomponent) " / 100")))
  (if (`/Game/Component/AC_Health.bIsDead` _healthcomponent)
    (`self.K2_DestroyActor` self)))

(fn `UserConstructionScript`)