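; Archery HUD that draws a crosshair reticle at screen center while the owning pawn is aiming.
; Each DrawHUD call finds the pawn's AC_Archery component and checks IsAiming before drawing.
; The reticle is four gapped arms sized by gap, length and thickness variables, drawn as a thicker dark pass under a white pass for an outline.
; An older plain-cross version remains in the graph, unconnected.
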(event `self.ReceiveDrawHUD`
  (params (SizeX :type Integer) (SizeY :type Integer))
  (bind _reticlegap (`self.ReticleGap`))
  (bind _reticlethickness (`self.ReticleThickness`))
  (bind _returnvalue (/ SizeX 2.0))
  (bind _returnvalue_2 (/ SizeY 2.0))
  (bind _returnvalue_3 (+ _reticlegap (`self.ReticleArmLength`)))
  (bind _asac_archery (cast `/Game/Component/Archery/AC_Archery` (`self.GetComponentByClass` (`self.GetOwningPawn`) "/Game/Component/Archery/AC_Archery.AC_Archery_C")))
  (bind _aiming (`/Game/Component/Archery/AC_Archery.IsAiming` _asac_archery))
  (if _aiming
    (`self.DrawLine` (- _returnvalue _returnvalue_3) _returnvalue_2 (- _returnvalue _reticlegap) _returnvalue_2 (struct :`A` 0.85) (+ _reticlethickness 2))
    (`self.DrawLine` (+ _returnvalue _reticlegap) _returnvalue_2 (+ _returnvalue _returnvalue_3) _returnvalue_2 (struct :`A` 0.85) (+ _reticlethickness 2))
    (`self.DrawLine` _returnvalue (- _returnvalue_2 _returnvalue_3) _returnvalue (- _returnvalue_2 _reticlegap) (struct :`A` 0.85) (+ _reticlethickness 2))
    (`self.DrawLine` _returnvalue (+ _returnvalue_2 _reticlegap) _returnvalue (+ _returnvalue_2 _returnvalue_3) (struct :`A` 0.85) (+ _reticlethickness 2))
    (`self.DrawLine` (- _returnvalue _returnvalue_3) _returnvalue_2 (- _returnvalue _reticlegap) _returnvalue_2 (struct :`R` 1 :`G` 1 :`B` 1 :`A` 1) _reticlethickness)
    (`self.DrawLine` (+ _returnvalue _reticlegap) _returnvalue_2 (+ _returnvalue _returnvalue_3) _returnvalue_2 (struct :`R` 1 :`G` 1 :`B` 1 :`A` 1) _reticlethickness)
    (`self.DrawLine` _returnvalue (- _returnvalue_2 _returnvalue_3) _returnvalue (- _returnvalue_2 _reticlegap) (struct :`R` 1 :`G` 1 :`B` 1 :`A` 1) _reticlethickness)
    (`self.DrawLine` _returnvalue (+ _returnvalue_2 _reticlegap) _returnvalue (+ _returnvalue_2 _returnvalue_3) (struct :`R` 1 :`G` 1 :`B` 1 :`A` 1) _reticlethickness)))

(fn `UserConstructionScript`)