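; Actor component that adds bow aiming and arrow firing to the sandbox player character, gated by death, ragdoll, roll, input and traversal state.
; TryFire checks a cooldown and muzzle obstruction, then launches an arrow projectile from a socket or offset toward a camera-traced aim point.
; A camera modifier registered at BeginPlay is handed this component, whose UpdateAimView blends to a collision-tested over-the-shoulder view and aim FOV.
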(event `self.ReceiveBeginPlay`
  (bind _assandbox_character_cmc (cast `/Game/Blueprints/SandboxCharacter_CMC` (`self.GetOwner`)))
  (set `self.PlayerCharacter` _assandbox_character_cmc)
  (bind _returnvalue (`PlayerCameraManager.AddNewCameraModifier` (`GameplayStatics.GetPlayerCameraManager` 0) "/Game/Component/Archery/BP_ArcheryCameraModifier.BP_ArcheryCameraModifier_C"))
  (bind _asbp_archery_camera_modifier (cast `/Game/Component/Archery/BP_ArcheryCameraModifier` _returnvalue))
  (set `/Game/Component/Archery/BP_ArcheryCameraModifier.Archery` self _asbp_archery_camera_modifier))

(fn `CanShoot`
  (returns (Allowed :type Boolean))
  (bind _playercharacter (`self.PlayerCharacter`))
  (bind _ac_combat (`/Game/Blueprints/SandboxCharacter_CMC.AC_Combat` _playercharacter))
  (`/Engine/EditorBlueprintResources/StandardMacros.IsValid` _playercharacter
    (:`Is Valid`
      (return (and (and (not (`/Game/Component/AC_Health.bIsDead` (`/Game/Blueprints/SandboxCharacter_CMC.HealthComponent` _playercharacter))) (not (`/Game/Blueprints/SandboxCharacter_CMC.IsRagdolling` _playercharacter))) (and (not (`/Game/Component/AC_Combat.IsRolling` _ac_combat)) (and (`/Game/Component/AC_Combat.inputEnabled` _ac_combat) (not (`/Game/Blueprints/AC_TraversalLogic.DoingTraversalAction` (`/Game/Blueprints/SandboxCharacter_CMC.AC_TraversalLogic` _playercharacter))))))))
    (:`Is Not Valid`
      (return false))))

(fn `ConfigureAimRotation`
  (bind _aiming (`self.IsAiming`))
  (if _aiming
    (set `CharacterMovementComponent.RotationRate` (`KismetMathLibrary.MakeRotator` 0.0 0.0 (`self.AimTurnSpeed`)) (`Character.CharacterMovement` (`self.PlayerCharacter`)))))

(fn `GetLaunchPosition`
  (returns (Position :type "Vector Structure"))
  (bind _playercharacter (`self.PlayerCharacter`))
  (bind _arrowlaunchorigin (`/Game/Blueprints/SandboxCharacter_CMC.ArrowLaunchOrigin` _playercharacter))
  (bind _mesh (`Character.Mesh` _playercharacter))
  (if (and (`self.UseMuzzleSocket`) (`SceneComponent.DoesSocketExist` _mesh (`self.MuzzleSocket`)))
    (return (`SceneComponent.GetSocketLocation` _mesh (`self.MuzzleSocket`)))
    (else
      (`SceneComponent.K2_SetWorldLocation` _arrowlaunchorigin (+ (`Actor.K2_GetActorLocation` _playercharacter) (`KismetMathLibrary.GreaterGreater_VectorRotator` (`self.LaunchOffset`) (`KismetMathLibrary.MakeRotator` 0.0 0.0 (.yaw (`PlayerCameraManager.GetCameraRotation` (`GameplayStatics.GetPlayerCameraManager` 0)))))) false true)
      (return (`SceneComponent.K2_GetComponentLocation` _arrowlaunchorigin)))))

(fn `IsAiming`
  (returns (Aiming :type Boolean))
  (bind _allowed (`self.CanShoot`))
  (return (and (`self.AimHeld`) _allowed)))

(fn `ResolveAim`
  (params (Origin :type "Vector Structure"))
  (returns (Direction :type "Vector Structure"))
  (bind _returnvalue (`GameplayStatics.GetPlayerCameraManager` 0))
  (bind _returnvalue_2 (`PlayerCameraManager.GetCameraLocation` _returnvalue))
  (bind _returnvalue_3 (+ _returnvalue_2 (* (`KismetMathLibrary.GetForwardVector` (`PlayerCameraManager.GetCameraRotation` _returnvalue)) (`self.AimTraceRange`))))
  (bind (_outhit _returnvalue_4) (`KismetSystemLibrary.LineTraceSingle` _returnvalue_2 _returnvalue_3 "TraceTypeQuery1" true (`|MakeArray` (`self.PlayerCharacter`) :!type "Actor Object Reference")))
  (return (`KismetMathLibrary.Normal` (- (select `bool` _returnvalue_4 :`false` _returnvalue_3 :`true` (`.ImpactPoint` (`GameplayStatics.BreakHitResult` _outhit))) Origin))))

(fn `SetAimHeld`
  (params (Held :type Boolean))
  (set `self.AimHeld` Held))

(fn `TryFire`
  (bind _playercharacter (`self.PlayerCharacter`))
  (bind _aiming (`self.IsAiming`))
  (if (and _aiming (>= (`GameplayStatics.GetTimeSeconds`) (`self.NextFireTime`)))
    (bind _position (`self.GetLaunchPosition`))
    (bind (_outhit _returnvalue) (`KismetSystemLibrary.SphereTraceSingle` (+ (`Actor.K2_GetActorLocation` _playercharacter) (`KismetMathLibrary.MakeVector` 0.0 0.0 (.z (`self.LaunchOffset`)))) _position 3.5 "TraceTypeQuery1" false (`|MakeArray` _playercharacter :!type "Actor Object Reference")))
    (set `self.LastMuzzleBlocked` _returnvalue)
    (if (not _returnvalue)
      (bind _direction (`self.ResolveAim` _position))
      (bind _returnvalue_2 (`|SpawnActorFromClass` "/Game/Component/Archery/BP_ArrowProjectile.BP_ArrowProjectile_C" (`KismetMathLibrary.MakeTransform` _position (`KismetMathLibrary.MakeRotFromX` _direction) (`KismetMathLibrary.MakeVector` 1.0 1.0 1.0)) "AlwaysSpawn" "MultiplyWithRoot" _playercharacter null))
      (`/Engine/EditorBlueprintResources/StandardMacros.IsValid` _returnvalue_2
        (:`Is Valid`
          (`/Game/Component/Archery/BP_ArrowProjectile.Launch` _returnvalue_2 _direction (`self.LaunchSpeed`) (`self.ArrowGravity`) (`self.ArrowDamage`) _playercharacter)
          (set `self.NextFireTime` (+ (`GameplayStatics.GetTimeSeconds`) (select `bool` (> (`self.FireInterval`) 0.05) :`false` 0.05 :`true` (`self.FireInterval`)))))))))

(fn `UpdateAimView`
  (params (DeltaTime :type "Float (double-precision)") (ViewLocation :type "Vector Structure") (ViewRotation :type "Rotator Structure") (FOV :type "Float (double-precision)"))
  (returns (NewLocation :type "Vector Structure") (NewRotation :type "Rotator Structure") (NewFOV :type "Float (double-precision)"))
  (bind _camerablend (`self.CameraBlend`))
  (bind _returnvalue (select `bool` (`self.OverrideNormalFOV`) :`false` FOV :`true` (`self.NormalFOV`)))
  (bind _returnvalue_2 (+ (`Actor.K2_GetActorLocation` (`self.PlayerCharacter`)) (`KismetMathLibrary.MakeVector` 0.0 0.0 (`self.AimCameraHeight`))))
  (bind _returnvalue_3 (`KismetMathLibrary.VLerp` ViewLocation (+ _returnvalue_2 (`KismetMathLibrary.GreaterGreater_VectorRotator` (`KismetMathLibrary.MakeVector` (- 0.0 (`self.AimCameraDistance`)) (`self.AimCameraShoulder`)) ViewRotation)) _camerablend))
  (set `self.LastBaseFOV` FOV)
  (bind _aiming (`self.IsAiming`))
  (bind _returnvalue_4 (`KismetMathLibrary.FInterpTo` (`self.CameraBlend`) (select `bool` _aiming :`false` 0.0 :`true` 1.0) DeltaTime (`self.CameraInterpSpeed`)))
  (set `self.CameraBlend` (select `bool` (< _returnvalue_4 0.001) :`false` (select `bool` (> _returnvalue_4 0.999) :`false` _returnvalue_4 :`true` 1.0) :`true` 0.0))
  (if (> _camerablend 0.0)
    (bind (_outhit _returnvalue_5) (`KismetSystemLibrary.SphereTraceSingle` _returnvalue_2 _returnvalue_3 (`self.CameraCollisionRadius`) "TraceTypeQuery2" false (`|MakeArray` (`self.PlayerCharacter`) :!type "Actor Object Reference")))
    (set `self.LastCameraBlocked` _returnvalue_5)
    (return (select `bool` _returnvalue_5 :`false` _returnvalue_3 :`true` (`.Location` (`GameplayStatics.BreakHitResult` _outhit))) ViewRotation (`KismetMathLibrary.Lerp` _returnvalue (`self.AimFOV`) _camerablend))
    (else
      (set `self.LastCameraBlocked` false)
      (return ViewLocation ViewRotation _returnvalue))))