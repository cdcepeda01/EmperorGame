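; Arrow projectile for archery, fired through Launch with direction, speed, gravity, damage and shooter, using a projectile movement component and query-only collision.
; When the projectile stops, a single guarded impact freezes it and attaches it to the hit component for a limited lifetime.
; Hits on BP_EnemyGASP_Ragdoll instead embed it at the closest physics-asset bone, falling back to nearest bone, clear its lifespan and apply point damage.
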(event `self.ArrowMovement.OnProjectileStop`
  (params (ImpactResult :type "HitResult Structure (by ref)"))
  (`self.HandleImpact` ImpactResult))

(fn `EmbedInEnemy`
  (params (Enemy :type "/Game/Component/BP_EnemyGASP_Ragdoll Object Reference") (Point :type "Vector Structure"))
  (bind _skeletalmesh (`/Game/Blueprints/SandboxCharacter_Mover.SkeletalMesh` Enemy))
  (bind (_closestworldposition _normal _bonename _distance _returnvalue) (`SkeletalMeshComponent.K2_GetClosestPointOnPhysicsAsset` _skeletalmesh Point))
  (set `self.HitBone` (select `bool` _returnvalue :`false` (`.ReturnValue` (`SkinnedMeshComponent.FindClosestBone_K2` _skeletalmesh Point 0.0 true)) :`true` _bonename))
  (set `self.ImpactComponent` _skeletalmesh)
  (`self.K2_SetActorLocation` self (+ (select `bool` _returnvalue :`false` Point :`true` _closestworldposition) (* (`self.FlightDirection`) (`self.EmbedDepth`))) false true)
  (`self.K2_AttachToComponent` self _skeletalmesh (`self.HitBone`) "KeepWorld" "KeepWorld" "KeepWorld" false)
  (`self.SetLifeSpan` self 0.0))

(fn `HandleImpact`
  (params (Impact :type "HitResult Structure"))
  (bind (_bblockinghit _binitialoverlap _time _distance _location _impactpoint _normal _impactnormal _physmat _hitactor _hitcomponent _hitbonename) (`GameplayStatics.BreakHitResult` Impact))
  (if (not (`self.HasImpacted`))
    (set `self.HasImpacted` true)
    (set `self.LastImpact` Impact)
    (set `self.ImpactComponent` _hitcomponent)
    (set `self.HitBone` _hitbonename)
    (`MovementComponent.StopMovementImmediately` (`self.ArrowMovement`))
    (`ActorComponent.Deactivate` (`self.ArrowMovement`))
    (`PrimitiveComponent.SetCollisionEnabled` (`self.ArrowCollision`) "NoCollision")
    (`self.SetLifeSpan` self (`self.EmbeddedLifetime`))
    (`/Engine/EditorBlueprintResources/StandardMacros.IsValid` _hitcomponent
      (:`Is Valid`
        (bind _asbp_enemy_gasp_ragdoll (cast `/Game/Component/BP_EnemyGASP_Ragdoll` _hitactor)
          (:`then`
            (`self.EmbedInEnemy` _asbp_enemy_gasp_ragdoll _impactpoint)
            (`GameplayStatics.ApplyPointDamage` _asbp_enemy_gasp_ragdoll (`self.ArrowDamage`) (`self.FlightDirection`) Impact (`Pawn.GetController` (`self.Shooter`)) self "/Script/Engine.DamageType"))
          (:`CastFailed`
            (`self.K2_AttachToComponent` self _hitcomponent _hitbonename "KeepWorld" "KeepWorld" "KeepWorld" false)))))))

(fn `Launch`
  (params (Direction :type "Vector Structure") (Speed :type "Float (double-precision)") (Gravity :type "Float (double-precision)") (Damage :type "Float (double-precision)") (SourcePawn :type "Pawn Object Reference"))
  (bind _arrowcollision (`self.ArrowCollision`))
  (bind _arrowmovement (`self.ArrowMovement`))
  (set `self.Shooter` SourcePawn)
  (set `self.ArrowDamage` Damage)
  (set `self.FlightSpeed` Speed)
  (set `self.GravityScale` Gravity)
  (set `self.FlightDirection` (`KismetMathLibrary.Normal` Direction))
  (`PrimitiveComponent.SetCollisionEnabled` (`self.ArrowMesh`) "NoCollision")
  (`PrimitiveComponent.SetCollisionObjectType` _arrowcollision "ECC_WorldDynamic")
  (`PrimitiveComponent.SetCollisionResponseToAllChannels` _arrowcollision "ECR_Block")
  (`PrimitiveComponent.SetCollisionResponseToChannel` _arrowcollision "ECC_Camera" "ECR_Ignore")
  (`PrimitiveComponent.SetCollisionResponseToChannel` _arrowcollision "ECC_Visibility" "ECR_Ignore")
  (`PrimitiveComponent.IgnoreActorWhenMoving` _arrowcollision SourcePawn true)
  (`PrimitiveComponent.SetCollisionEnabled` _arrowcollision "QueryOnly")
  (`MovementComponent.SetUpdatedComponent` _arrowmovement _arrowcollision)
  (set `ProjectileMovementComponent.ProjectileGravityScale` Gravity _arrowmovement)
  (set `MovementComponent.Velocity` (* (`self.FlightDirection`) Speed) _arrowmovement)
  (`ActorComponent.Activate` _arrowmovement true)
  (`self.SetLifeSpan` self 8.0))

(fn `UserConstructionScript`
  (`PrimitiveComponent.SetCollisionEnabled` (`self.ArrowMesh`) "NoCollision")
  (`PrimitiveComponent.SetCollisionEnabled` (`self.ArrowCollision`) "NoCollision"))