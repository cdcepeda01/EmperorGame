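; AI controller for BP_EnemyGASP_Ragdoll enemies that roams around the possession point, chases the player and triggers attacks.
; A looping UpdateAI timer replaces Tick, halting movement while dead, hit-reacting or attacking, otherwise updating senses and choosing Chase or Roam.
; Hand-rolled sight combines distance, facing dot product and line of sight, retaining the target briefly after losing sight.
; Chase heads for the visible player or last seen location; Roam picks random reachable navmesh points.
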(event `self.ReceiveBeginPlay`
  (`KismetSystemLibrary.K2_SetTimer` self "UpdateAI" 0.2 true))

(event `self.ReceivePossess`
  (params (PossessedPawn :type "Pawn Object Reference"))
  (set `self.HomeLocation` (`self.K2_GetActorLocation` PossessedPawn)))

(event `self.ReceiveUnPossess`
  (params (UnpossessedPawn :type "Pawn Object Reference"))
  (`self.StopMovement`)
  (`KismetSystemLibrary.K2_ClearTimer` self "UpdateAI"))

(fn `Chase`
  (bind _asbp_enemy_gasp_ragdoll (cast `/Game/Component/BP_EnemyGASP_Ragdoll` (`self.K2_GetPawn`)))
  (if (`self.CanSeePlayer`)
    (if (<= (`self.GetDistanceTo` _asbp_enemy_gasp_ragdoll (`self.TargetPawn`)) (`/Game/Component/BP_EnemyGASP_Ragdoll.AttackRange` _asbp_enemy_gasp_ragdoll))
      (`self.StopMovement`)
      (`/Game/Component/BP_EnemyGASP_Ragdoll.TryEnemyAttack` _asbp_enemy_gasp_ragdoll (`self.TargetPawn`))
      (else
        (`self.MoveToActor` (`self.TargetPawn`) (`self.ChaseAcceptanceRadius`) true true false null)))
    (else
      (`self.MoveToLocation` (`self.LastSeenLocation`) 90.0 true true true false null))))

(fn `Roam`
  (switch `EPathFollowingStatus` (`self.GetMoveStatus`)
    (:`Idle`
      (if (>= (`GameplayStatics.GetTimeSeconds`) (`self.NextRoamTime`))
        (bind (_destination _found) (`self.SampleRoamPoint`))
        (set `self.NextRoamTime` (+ (`GameplayStatics.GetTimeSeconds`) 2.0))
        (if _found
          (set `self.RoamDestination` _destination)
          (`self.MoveToLocation` (`self.RoamDestination`) 65.0 true true false false null false))))))

(fn `SampleRoamPoint`
  (returns (Destination :type "Vector Structure") (Found :type Boolean))
  (bind (_randomlocation _returnvalue) (`NavigationSystemV1.K2_GetRandomReachablePointInRadius` (`self.HomeLocation`) (`self.RoamRadius`) null null))
  (return _randomlocation _returnvalue))

(fn `UpdateAI`
  (bind _asbp_enemy_gasp_ragdoll (cast `/Game/Component/BP_EnemyGASP_Ragdoll` (`self.K2_GetPawn`))
    (:`then`
      (bind (_result _reactingtohit _attacking) (`/Game/Component/BP_EnemyGASP_Ragdoll.IsEnemyDead` _asbp_enemy_gasp_ragdoll))
      (if _result
        (`self.StopMovement`)
        (set `self.State` "Dead")
        (`KismetSystemLibrary.K2_ClearTimer` self "UpdateAI")
        (elif _reactingtohit
          (`self.StopMovement`)
          (set `self.State` "HitReaction")
          (elif _attacking
            (`self.StopMovement`)
            (set `self.State` "Attacking")
            (else
              (`self.UpdateSenses`)
              (`/Engine/EditorBlueprintResources/StandardMacros.IsValid` (`self.TargetPawn`)
                (:`Is Valid`
                  (set `self.State` "Chasing")
                  (`self.Chase`))
                (:`Is Not Valid`
                  (if (`KismetStringLibrary.EqualEqual_StrStr` (`self.State`) "Chasing")
                    (`self.StopMovement`))
                  (set `self.State` "Roaming")
                  (`self.Roam`))))))))
    (:`CastFailed`
      (`self.StopMovement`))))

(fn `UpdateSenses`
  (bind _returnvalue (`GameplayStatics.GetPlayerPawn` 0))
  (bind _returnvalue_2 (`self.K2_GetPawn`))
  (set `self.CanSeePlayer` false)
  (`/Engine/EditorBlueprintResources/StandardMacros.IsValid` _returnvalue
    (:`Is Valid`
      (if (and (not (`/Game/Component/AC_Health.bIsDead` (`self.GetComponentByClass` _returnvalue "/Game/Component/AC_Health.AC_Health_C"))) (and (<= (`self.GetDistanceTo` _returnvalue_2 _returnvalue) (`self.SightRadius`)) (and (>= (`self.GetHorizontalDotProductTo` _returnvalue_2 _returnvalue) (`self.SightDotThreshold`)) (`self.LineOfSightTo` _returnvalue))))
        (set `self.CanSeePlayer` true)
        (set `self.TargetPawn` _returnvalue)
        (set `self.LastSeenTime` (`GameplayStatics.GetTimeSeconds`))
        (set `self.LastSeenLocation` (`self.K2_GetActorLocation` _returnvalue))
        (elif (> (- (`GameplayStatics.GetTimeSeconds`) (`self.LastSeenTime`)) (`self.LoseSightDelay`))
          (set `self.TargetPawn` null))))
    (:`Is Not Valid`
      (set `self.TargetPawn` null))))

(fn `UserConstructionScript`)