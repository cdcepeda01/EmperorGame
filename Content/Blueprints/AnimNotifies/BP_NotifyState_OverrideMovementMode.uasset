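; Anim notify state that temporarily switches a SandboxCharacter_Mover's movement mode for a section of an animation.
; On begin it queues the override mode on the owner's Mover component.
; On end it queues the ending mode, but only if the override mode is still active, so a mode change made elsewhere during the window is left intact.
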(fn `Received_NotifyBegin`
  (params (MeshComp :type "SkeletalMeshComponent Object Reference") (Animation :type "AnimSequenceBase Object Reference") (TotalDuration :type "Float (single-precision)") (EventReference :type "AnimNotifyEventReference Structure (by ref)"))
  (returns (ReturnValue :type Boolean))
  (bind _assandbox_character_mover (cast `/Game/Blueprints/SandboxCharacter_Mover` (`ActorComponent.GetOwner` MeshComp)))
  (`MoverComponent.QueueNextMode` (`/Game/Blueprints/SandboxCharacter_Mover.CharacterMover` _assandbox_character_mover) (`self.OverrideMovementMode`) false)
  (return false))

(fn `Received_NotifyEnd`
  (params (MeshComp :type "SkeletalMeshComponent Object Reference") (Animation :type "AnimSequenceBase Object Reference") (EventReference :type "AnimNotifyEventReference Structure (by ref)"))
  (returns (ReturnValue :type Boolean))
  (bind _assandbox_character_mover (cast `/Game/Blueprints/SandboxCharacter_Mover` (`ActorComponent.GetOwner` MeshComp)))
  (bind _charactermover (`/Game/Blueprints/SandboxCharacter_Mover.CharacterMover` _assandbox_character_mover))
  (if (== (`MoverComponent.GetMovementModeName` _charactermover) (`self.OverrideMovementMode`))
    (`MoverComponent.QueueNextMode` _charactermover (`self.EndingMovementMode`) false)
    (return false)))