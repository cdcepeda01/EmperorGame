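; Flying movement mode that generates each move's velocity and rotation from desired velocity and facing.
; GenerateFlyingMove smooths the current velocity toward the desired velocity with DampVector over a short fixed smoothing time.
; It also damps the current facing toward the desired facing with DampQuat, then converts that rotation step into angular velocity in degrees, writing both results back through by-ref outputs.
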(fn `GenerateFlyingMove`
  (params (StartState :type "MoverTickStartData Structure (by ref)") (DeltaSeconds :type "Float (single-precision)") (DesiredVelocity :type "Vector Structure (by ref)") (DesiredFacing :type "Quat Structure (by ref)") (CurrentFacing :type "Quat Structure (by ref)") (InOutAngularVelocityDegrees :type "Vector Structure (by ref)") (InOutVelocity :type "Vector Structure (by ref)"))
  (locals (`Angular Velocity Radians` :type "Vector Structure"))
  (`|ExecutionSequence`
    (:`then_0`
      (`|VariableSetRef` (`local.InOutVelocity`) (`BlueprintSpringMathLibrary.DampVector` (`local.InOutVelocity`) (`local.DesiredVelocity`) (`local.DeltaSeconds`) 0.1)))
    (:`then_1`
      (bind _returnvalue (`MovementUtils.ComputeAngularVelocityDegrees` (`KismetMathLibrary.Quat_Rotator` (`local.CurrentFacing`)) (`KismetMathLibrary.Quat_Rotator` (`BlueprintSpringMathLibrary.DampQuat` (`local.CurrentFacing`) (`local.DesiredFacing`) (`local.DeltaSeconds`))) (`local.DeltaSeconds`)))
      (`|VariableSetRef` (`local.InOutAngularVelocityDegrees`) _returnvalue))))